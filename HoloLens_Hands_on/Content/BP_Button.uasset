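; BP_Button is an actor that wraps a UX Tools pressable button and spawns physics cubes when pressed.
; On BeginPlay it casts its child actor to UxtPressableButtonActor and binds to the button component's pressed event.
; Each press spawns a scaled-down BP_PhysicsCube at the actor's own location and rotation, with a limited lifespan so cubes clean themselves up.
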(event Custom|OnButtonPressed
  (params (Button :type Uxt%20Pressable%20Button%20Component%20Object%20Reference) (Pointer :type Uxt%20Pointer%20Component%20Object%20Reference))
  (bind _returnvalue (Transformation|GetActorTransform))
  (bind (_location _rotation) (Math|Transform|BreakTransform _returnvalue))
  (bind _returnvalue_2 (Game|SpawnActorfromClass "/Game/BP_PhysicsCube.BP_PhysicsCube_C" (Math|Transform|MakeTransform _location _rotation "0.300000,0.300000,0.300000") "Undefined" 0 0))
  (Actor|SetLifeSpan _returnvalue_2 6e+01))

(event EventBeginPlay
  (bind _asuxt_pressable_button_actor (Utilities|Casting|CastToUxtPressableButtonActor (Variables|/Script/Engine.ChildActorComponent|GetChildActor (Variables|Default|GetChildActor))))
  (EventDispatchers|BindEventtoOnButtonPressed (Variables|/Script/UXTools.UxtBasePressableButtonActor|GetButtonComponent _asuxt_pressable_button_actor) (delegate Custom|OnButtonPressed)))

(event Collision|EventActorBeginOverlap
  (params (OtherActor :type Actor%20Object%20Reference)))

(event EventTick
  (params (DeltaSeconds :type Float%20%28single-precision%29)))

(fn ConstructionScript)